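; Block_BP is a 2D Paper2D ground block carrying an enemy, which the player scores on by passing.
; On BeginPlay it builds a grid of sprite tiles with random width and fixed depth, then places the enemy at a random X along the top.
; Overlapping either the block or enemy trigger adds to MyPlayer's score and destroys the block after a delay.
; Hitting the enemy's collision starts the player's death sequence unless already dead.
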(event `self.ReceiveBeginPlay`
  ;[1 1 1] Begin Play Event
  (`|ExecutionSequence`
    (:`then_0`
      (set `self.HorTiles` (`KismetMathLibrary.RandomIntegerInRange` 6 10))
      (set `self.VerTiles` 10)
      (for _index (range (+ (`self.HorTiles`) 1))
        (bind _returnvalue (* _index 100.0))
        (`AddComponent|PaperSpriteComponent_40` :`RelativeTransform` (`KismetMathLibrary.MakeTransform` (`KismetMathLibrary.MakeVector` _returnvalue)))
        (for _index_2 (range 1 (+ (`self.VerTiles`) 1))
          (`AddComponent|PaperSpriteComponent_43` :`RelativeTransform` (`KismetMathLibrary.MakeTransform` (`KismetMathLibrary.MakeVector` _returnvalue 0.0 (* _index_2 -100.0)))))))
    (:`then_1`
      (`SceneComponent.K2_SetRelativeLocation` (`self.Enemy_Anim`) (`KismetMathLibrary.MakeVector` (* (`KismetMathLibrary.RandomFloat`) (* (`self.HorTiles`) 100.0)) 0.0 50.0) false false))))

(event `self.Enemy_trigger.OnComponentBeginOverlap`
  (params (OverlappedComponent :type "PrimitiveComponent Object Reference") (OtherActor :type "Actor Object Reference") (OtherComp :type "PrimitiveComponent Object Reference") (OtherBodyIndex :type Integer) (bFromSweep :type Boolean) (SweepResult :type "HitResult Structure (by ref)"))
  (bind _asmy_player (cast `/Game/Blueprints/MyPlayer` OtherActor))
  (`/Game/Blueprints/MyPlayer.UpdateScore` _asmy_player 1)
  (`KismetSystemLibrary.Delay` 10.0)
  (`self.K2_DestroyActor`))

(event `self.Trigger.OnComponentBeginOverlap`
  (params (OverlappedComponent :type "PrimitiveComponent Object Reference") (OtherActor :type "Actor Object Reference") (OtherComp :type "PrimitiveComponent Object Reference") (OtherBodyIndex :type Integer) (bFromSweep :type Boolean) (SweepResult :type "HitResult Structure (by ref)"))
  ;[1 1 1] Player Scoring Trigger Overlaping
  (bind _asmy_player (cast `/Game/Blueprints/MyPlayer` OtherActor))
  (`/Game/Blueprints/MyPlayer.UpdateScore` _asmy_player 1)
  (`KismetSystemLibrary.Delay` 10.0)
  (`self.K2_DestroyActor`))

(event `self.Enemy_Collision.OnComponentHit`
  (params (HitComponent :type "PrimitiveComponent Object Reference") (OtherActor :type "Actor Object Reference") (OtherComp :type "PrimitiveComponent Object Reference") (NormalImpulse :type "Vector Structure") (Hit :type "HitResult Structure (by ref)"))
  ;[1 1 1] Player/Enemy Overlapping
  (bind _asmy_player (cast `/Game/Blueprints/MyPlayer` OtherActor))
  (if (not (`/Game/Blueprints/MyPlayer.isDead` _asmy_player))
    (`/Game/Blueprints/MyPlayer.DeathSequence` _asmy_player)))

(fn `UserConstructionScript`)